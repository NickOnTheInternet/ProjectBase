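; Player character Blueprint that handles basic movement, look and crouch through Enhanced Input.
; On BeginPlay it casts the first player controller to BP_PC_Game and adds the IMC_Default mapping context to its input subsystem.
; Move input drives movement along the actor's right and forward vectors, and look input feeds controller yaw and pitch.
; The crouch action works as a toggle based on the current crouched state.
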(event `self.ReceiveBeginPlay`
  (bind _asbp_pc_game (cast `/Game/Game/Blueprints/Core/BP_PC_Game` (`GameplayStatics.GetPlayerController` 0)))
  (bind _returnvalue (pcsubsystem `EnhancedInputLocalPlayerSubsystem` _asbp_pc_game))
  (`/Engine/EditorBlueprintResources/StandardMacros.IsValid` _returnvalue
    (:`Is Valid`
      (`EnhancedInputSubsystemInterface.AddMappingContext` _returnvalue "/Game/Game/Blueprints/Input/IMC_Default.IMC_Default" 0 (struct)))))

(event `EnhancedInput|/Game/Game/Blueprints/Input/IA_Move`
  (params (ActionValue :type "Vector2D Structure") (ElapsedSeconds :type "Float (double-precision)") (TriggeredSeconds :type "Float (double-precision)") (InputAction :type "InputAction Object Reference" :default "/Game/Game/Blueprints/Input/IA_Move.IA_Move"))
  (:`Triggered`
    (`self.AddMovementInput` (`self.GetActorRightVector`) ActionValue_X)
    (`self.AddMovementInput` (`self.GetActorForwardVector`) ActionValue_Y)))

(event `EnhancedInput|/Game/Game/Blueprints/Input/IA_Look`
  (params (ActionValue :type "Vector2D Structure") (ElapsedSeconds :type "Float (double-precision)") (TriggeredSeconds :type "Float (double-precision)") (InputAction :type "InputAction Object Reference" :default "/Game/Game/Blueprints/Input/IA_Look.IA_Look"))
  (:`Triggered`
    (`self.AddControllerYawInput` ActionValue_X)
    (`self.AddControllerPitchInput` ActionValue_Y)))

(event `EnhancedInput|/Game/Game/Blueprints/Input/IA_Crouch`
  (params (ActionValue :type Boolean) (ElapsedSeconds :type "Float (double-precision)") (TriggeredSeconds :type "Float (double-precision)") (InputAction :type "InputAction Object Reference" :default "/Game/Game/Blueprints/Input/IA_Crouch.IA_Crouch"))
  (:`Triggered`
    (if (`self.bIsCrouched`)
      (`self.UnCrouch`)
      (else
        (`self.Crouch`)))))

(fn `UserConstructionScript`
  (`parent.UserConstructionScript`))